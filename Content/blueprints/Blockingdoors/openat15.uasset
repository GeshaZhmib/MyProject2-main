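; A blocking door actor that removes itself at a set game time, with a tutorial widget for the player.
; Each tick it sets its Cube visible only in scene captures and destroys the actor once the game instance's Time reaches Opensat.
; The widget starts hidden and shows only while the first-person character overlaps the Trigger.
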(event `self.ReceiveTick`
  (params (DeltaSeconds :type "Float (single-precision)"))
  (bind _asgi_main (cast `/Game/blueprints/gi_main` (`GameplayStatics.GetGameInstance`)))
  ;[1 1 1] блок пропадает в игре в какое-тоопределенное время
  (`PrimitiveComponent.SetVisibleInSceneCaptureOnly` (`self.Cube`) true)
  (if (>= (`/Game/blueprints/gi_main.time` _asgi_main) (`self.opensat`))
    (`self.K2_DestroyActor`)))

(event `self.trigger.OnComponentBeginOverlap`
  (params (OverlappedComponent :type "PrimitiveComponent Object Reference") (OtherActor :type "Actor Object Reference") (OtherComp :type "PrimitiveComponent Object Reference") (OtherBodyIndex :type Integer) (bFromSweep :type Boolean) (SweepResult :type "HitResult Structure (by ref)"))
  ;[1 1 1] tutorial
  (cast `/Game/blueprints/1stCharBP` OtherActor)
  (`SceneComponent.SetVisibility` (`self.Widget`) true false))

(event `self.trigger.OnComponentEndOverlap`
  (params (OverlappedComponent :type "PrimitiveComponent Object Reference") (OtherActor :type "Actor Object Reference") (OtherComp :type "PrimitiveComponent Object Reference") (OtherBodyIndex :type Integer))
  ;[1 1 1] tutorial
  (cast `/Game/blueprints/1stCharBP` OtherActor)
  (`SceneComponent.SetVisibility` (`self.Widget`) false false))

(fn `UserConstructionScript`
  (`SceneComponent.SetVisibility` (`self.Widget`) false false))