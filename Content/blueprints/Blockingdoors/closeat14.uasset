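; Time-gated blocking door that appears once the game time reaches a threshold, with a tutorial widget.
; Tick polls Time on gi_main, keeping the actor hidden without Cube collision until it reaches NewVar.
; From then on the actor is unhidden, with Cube set to query-only collision and visible only in scene captures.
; The widget starts hidden and shows while 1stCharBP overlaps Trigger.
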(event `self.ReceiveTick`
  (params (DeltaSeconds :type "Float (single-precision)"))
  ;[1 1 1] дверь исчезает
  (bind _asgi_main (cast `/Game/blueprints/gi_main` (`GameplayStatics.GetGameInstance`)))
  (`self.SetActorHiddenInGame` true)
  (`PrimitiveComponent.SetCollisionEnabled` (`self.Cube`) "NoCollision")
  (if (>= (`/Game/blueprints/gi_main.time` _asgi_main) (`self.NewVar`))
    (`self.SetActorHiddenInGame` false)
    (`PrimitiveComponent.SetVisibleInSceneCaptureOnly` (`self.Cube`) true)
    (`PrimitiveComponent.SetCollisionEnabled` (`self.Cube`) "QueryOnly")))

(event `self.trigger.OnComponentBeginOverlap`
  (params (OverlappedComponent :type "PrimitiveComponent Object Reference") (OtherActor :type "Actor Object Reference") (OtherComp :type "PrimitiveComponent Object Reference") (OtherBodyIndex :type Integer) (bFromSweep :type Boolean) (SweepResult :type "HitResult Structure (by ref)"))
  ;[1 1 1] туториал
  (cast `/Game/blueprints/1stCharBP` OtherActor)
  (`SceneComponent.SetVisibility` (`self.Widget`) true false))

(event `self.trigger.OnComponentEndOverlap`
  (params (OverlappedComponent :type "PrimitiveComponent Object Reference") (OtherActor :type "Actor Object Reference") (OtherComp :type "PrimitiveComponent Object Reference") (OtherBodyIndex :type Integer))
  ;[1 1 1] туториал
  (cast `/Game/blueprints/1stCharBP` OtherActor)
  (`SceneComponent.SetVisibility` (`self.Widget`) false false))

(fn `UserConstructionScript`
  (`SceneComponent.SetVisibility` (`self.Widget`) false false))