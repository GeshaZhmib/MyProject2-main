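; Blocking door actor that removes itself on a timer after play begins, with a proximity tutorial widget.
; On BeginPlay it makes its Cube visible only in scene captures, waits a fixed delay, then destroys the whole actor.
; The construction script hides the Widget, and the Trigger component shows it only while the first-person character overlaps.
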(event `self.ReceiveBeginPlay`
  ;[1 1 1] блок пропадает в игре в какое-тоопределенное время
  (`self.disapear`))

(event `disapear`
  ;[1 1 1] блок пропадает в игре в какое-тоопределенное время
  (`PrimitiveComponent.SetVisibleInSceneCaptureOnly` (`self.Cube`) true)
  (`KismetSystemLibrary.Delay` 8.0)
  (`self.K2_DestroyActor`))

(event `self.trigger.OnComponentBeginOverlap`
  (params (OverlappedComponent :type "PrimitiveComponent Object Reference") (OtherActor :type "Actor Object Reference") (OtherComp :type "PrimitiveComponent Object Reference") (OtherBodyIndex :type Integer) (bFromSweep :type Boolean) (SweepResult :type "HitResult Structure (by ref)"))
  ;[1 1 1] tutorial
  (cast `/Game/blueprints/1stCharBP` OtherActor)
  (`SceneComponent.SetVisibility` (`self.Widget`) true false))

(event `self.trigger.OnComponentEndOverlap`
  (params (OverlappedComponent :type "PrimitiveComponent Object Reference") (OtherActor :type "Actor Object Reference") (OtherComp :type "PrimitiveComponent Object Reference") (OtherBodyIndex :type Integer))
  ;[1 1 1] tutorial
  (cast `/Game/blueprints/1stCharBP` OtherActor)
  (`SceneComponent.SetVisibility` (`self.Widget`) false false))

(fn `UserConstructionScript`
  (`SceneComponent.SetVisibility` (`self.Widget`) false false))