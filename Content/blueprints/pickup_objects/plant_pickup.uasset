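; Plant pickup actor that the player collects through an Interact function.
; Interact fires the destroy event and returns the actor's static mesh to the caller.
; After a short delay, the event casts the player character to 1stCharBP, makes the Red element of its inventory visible, then destroys the actor.
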(event `destroy`
  (`KismetSystemLibrary.Delay` 0.2)
  (bind _as1st_char_bp (cast `/Game/blueprints/1stCharBP` (`GameplayStatics.GetPlayerCharacter` 0)))
  (`Widget.SetVisibility` (`/Game/UI/inventar/inveniry_widget.red` (`/Game/blueprints/1stCharBP.invenory` _as1st_char_bp)) "Visible")
  (`self.K2_DestroyActor`))

(fn `interact`
  (returns (plant :type "StaticMesh Object Reference"))
  (`self.destroy`)
  (return (`StaticMeshComponent.StaticMesh` (`self.StaticMesh`))))

(fn `UserConstructionScript`)