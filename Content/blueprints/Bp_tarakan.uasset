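; Bp_tarakan is a talkable Blueprint that shows its dialogue one line at a time through a Talk event.
; Each call increments Talkindex, creates the WB_diologue widget if none is valid, sets its text from the Dialogue array and plays a 2D sound.
; Once the index passes the last line, it removes the widget from its parent; the index is never reset here.
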(event `/Game/blueprints/BPI_diologtaracan.talk`
  (`/Engine/EditorBlueprintResources/StandardMacros.IncrementInt` (`self.talkindex`)
    (:`  `
      (if (< (`self.talkindex`) (`KismetArrayLibrary.Array_Length` (`self.dialogue`)))
        (`self.ui`
          (:`then`
            _)
          (:`else`
            (bind _returnvalue (`|CreateWidget` "/Game/blueprints/WB_diologue.WB_diologue_C" (`GameplayStatics.GetPlayerController` 0)))
            (bind _output_get (set `self.ui` _returnvalue))
            (`UserWidget.AddToViewport` _output_get 0)))
        (`TextBlock.SetText` (`/Game/blueprints/WB_diologue.talktextt` (`self.ui`)) (`KismetTextLibrary.Conv_StringToText` (`|GetArrayItem` (`self.dialogue`) (`self.talkindex`))))
        (`GameplayStatics.PlaySound2D` null 1.0 1.0 0.0 null null)
        (else
          (`Widget.RemoveFromParent` (`self.ui`)))))))

(fn `UserConstructionScript`)