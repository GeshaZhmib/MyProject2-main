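; An interactable "risunki" actor that shows lines of dialogue and grants the player an inventory item.
; A trigger toggles a widget's visibility, hidden by default, as the first-person character enters or leaves.
; Each Talk call advances through the Dialogue array in a WB_diologue UI with a sound and adds item 0 uniquely to the game instance's inventory.
; Once the lines run out, the dialogue UI is removed.
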(event `self.talk`
  (`/Engine/EditorBlueprintResources/StandardMacros.IncrementInt` (`self.talkindex`)
    (:`  `
      (if (< (`self.talkindex`) (`KismetArrayLibrary.Array_Length` (`self.dialogue`)))
        (`self.ui`
          (:`then`
            _)
          (:`else`
            (bind _returnvalue (`|CreateWidget` "/Game/blueprints/dialog/WB_diologue.WB_diologue_C" (`GameplayStatics.GetPlayerController` 0)))
            (bind _output_get (set `self.ui` _returnvalue))
            (`UserWidget.AddToViewport` _output_get 0)))
        (`TextBlock.SetText` (`/Game/blueprints/dialog/WB_diologue.talktextt` (`self.ui`)) (`KismetTextLibrary.Conv_StringToText` (`|GetArrayItem` (`self.dialogue`) (`self.talkindex`))))
        (`GameplayStatics.PlaySound2D` null 1.0 1.0 0.0 null null)
        (bind _asgi_main (cast `/Game/blueprints/gi_main` (`GameplayStatics.GetGameInstance`)))
        (`KismetArrayLibrary.Array_AddUnique` (`/Game/blueprints/gi_main.inventaryitems` _asgi_main))
        (else
          (`Widget.RemoveFromParent` (`self.ui`)))))))

(event `self.Triger.OnComponentBeginOverlap`
  (params (OverlappedComponent :type "PrimitiveComponent Object Reference") (OtherActor :type "Actor Object Reference") (OtherComp :type "PrimitiveComponent Object Reference") (OtherBodyIndex :type Integer) (bFromSweep :type Boolean) (SweepResult :type "HitResult Structure (by ref)"))
  (cast `/Game/blueprints/1stCharBP` OtherActor)
  (`SceneComponent.SetVisibility` (`self.Widget`) true false))

(event `self.Triger.OnComponentEndOverlap`
  (params (OverlappedComponent :type "PrimitiveComponent Object Reference") (OtherActor :type "Actor Object Reference") (OtherComp :type "PrimitiveComponent Object Reference") (OtherBodyIndex :type Integer))
  (cast `/Game/blueprints/1stCharBP` OtherActor)
  (`SceneComponent.SetVisibility` (`self.Widget`) false false))

(fn `UserConstructionScript`
  (`SceneComponent.SetVisibility` (`self.Widget`) false false))