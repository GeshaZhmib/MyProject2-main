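; Actor component that makes its owning Light actor flicker using selectable Quake-style letter-string patterns.
; On BeginPlay it caches the light component, or prints a warning and deactivates if the owner isn't a light.
; SetFlicker stores base intensity and starts a looping timer, or stops it and restores that intensity.
; Each tick of the timer maps the next letter to an intensity multiplier ('m' near normal) and calls OnLightUpdate.
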(event `self.ReceiveBeginPlay`
  (bind _aslight (cast `Light` (`self.GetOwner`))
    (:`then`
      (set `self.LightComponent` (`Light.LightComponent` _aslight))
      (`self.SetFlicker` (`self.bIsFlickering`)))
    (:`CastFailed`
      (`KismetSystemLibrary.PrintString` "Flicker light component is attached to something that isn't a light!")
      (`self.Deactivate`))))

(fn `CharacterToNumber`
  (params (String :type String) (Index :type Integer))
  (returns (Integer :type Integer))
  (return (`KismetMathLibrary.Clamp` (- (`KismetStringLibrary.GetCharacterAsNumber` String Index) 97) 0 26)))

(fn `FlickerStrings`
  (returns (Flicker :type String))
  (return (select `int` (`self.FlickerType`) :`0` "m" :`1` "mmmmmaaaaammmmmaaaaaabcdefgabcdefg" :`2` "abcdefghijklmnopqrstuvwxyzyxwvutsrqponmlkjihgfedcba" :`3` "mmmmmaaaaammmmmaaaaaabcdefgabcdefg" :`4` "mamamamamama" :`5` "jklmnopqrstuvwxyzyxwvutsrqponmlkj" :`6` "nmonqnmomnmomomno" :`7` "mmmaaaabcdefgmmmmaaaammmaamm" :`8` "mmmaaammmaaammmabcdefaaaammmmabcdefmmmaaaa" :`9` "aaaaaaaazzzzzzzz" :`10` "mmamammmmammamamaaamammma" :`11` "abcdefghijklmnopqrrqponmlkjihgfedcba")))

(fn `SetFlicker`
  (params (bIsFlickering :type Boolean))
  (bind _output_get (set `self.bIsFlickering` bIsFlickering))
  (if _output_get
    (set `self.BaseIntensity` (`LightComponentBase.Intensity` (`self.LightComponent`)))
    (`KismetSystemLibrary.K2_SetTimer` null "UpdateFlicker" (`self.Frequency`) true)
    (return)
    (else
      (`KismetSystemLibrary.K2_ClearTimer` null "UpdateFlicker")
      (`LightComponent.SetIntensity` (`self.LightComponent`) (`self.BaseIntensity`))
      (`self.OnLightUpdate` (`self.BaseIntensity`))
      (return))))

(fn `UpdateFlicker`
  (locals (String :type String))
  (set `local.String` (`self.FlickerStrings`))
  (`|ExecutionSequence`
    (:`then_0`
      ;[1 1 1] Set the intensity
      (`LightComponent.SetIntensity` (`self.LightComponent`) (* (/ (`KismetMathLibrary.Conv_IntToDouble` (`self.CharacterToNumber` (`local.String`) (`self.Step`))) 13.0) (`self.BaseIntensity`)))
      (`self.OnLightUpdate` (`LightComponentBase.Intensity` (`self.LightComponent`))))
    (:`then_1`
      (set `self.Step` (select `bool` (> (- (`KismetStringLibrary.Len` (`local.String`)) 1) (`self.Step`)) :`true` (+ (`self.Step`) 1)))
      (return))))